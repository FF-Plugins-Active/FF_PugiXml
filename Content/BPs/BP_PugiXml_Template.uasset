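; Test Blueprint for plugin functions wrapping libdeflate and pugixml.
; On BeginPlay it loads a .docx from a hardcoded local path, passes its bytes to LibDeflateTest, and prints the uncompressed buffer length or the error code through a callback.
; Unconnected graphs hold pugixml samples that create a document, add a node and print the XML, but they never run.
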(event Custom|CustomEvent
  (params (bIsSuccessful :type Boolean) (Out_Bytes :type Deflate%20Uncompressed%20Structure) (Out_Code :type String))
  (if bIsSuccessful
    (Development|PrintString (Utilities|String|ToString(Integer) (Utilities|Array|Length (.uncompressedbuffer Out_Bytes))) true true "(R=0.000000,G=1.000000,B=0.000000,A=1.000000)" 3e+01)
    (else
      (Development|PrintString Out_Code true true "(R=1.000000,G=0.000000,B=0.000000,A=1.000000)" 3e+01))))

(event EventBeginPlay
  (Class|FFPugiXmlBPLibrary|LibDeflateTest (delegate Custom|CustomEvent) (Class|LowEntryFileManagerLibrary|GetFileData (Class|KismetSystemLibrary|NormalizeFilename "C:\\Users\\erayo\\Downloads\\test.docx"))))

(fn ConstructionScript)